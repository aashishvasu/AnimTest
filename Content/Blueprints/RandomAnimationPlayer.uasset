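; Actor Blueprint that shows a randomly chosen skeletal mesh playing a random looping animation.
; All setup runs in the construction script, with the Randomize flag acting as a one-shot button that rolls a new RandomSeed.
; That stored seed drives the mesh pick, animation pick and slight play-rate variation, so each result is repeatable.
; The event graph has no logic.
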(event `Play`)

(fn `UserConstructionScript`
  (bind _skeletalmesh (`self.SkeletalMesh`))
  (if (`self.Randomize`)
    (set `self.Randomize` false)
    (set `self.RandomSeed` (`KismetMathLibrary.RandomIntegerInRange` 0 99999)))
  (`SkinnedMeshComponent.SetSkinnedAssetAndUpdate` _skeletalmesh (`self.GetRandomInArray` (`self.Meshes`) (`self.RandomSeed`)) true)
  (`SkeletalMeshComponent.SetAnimationMode` _skeletalmesh "AnimationSingleNode")
  (set `SkeletalMeshComponent.AnimationData` (make `SingleAnimationPlayData` (`self.GetRandomInArray` (`self.Anims`) (`self.RandomSeed`)) true true 0.0 (`KismetMathLibrary.RandomFloatInRangeFromStream` 0.9 1.1 (`KismetMathLibrary.MakeRandomStream` (`self.RandomSeed`)))) _skeletalmesh))